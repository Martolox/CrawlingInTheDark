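; Room camera for a Paper2D character that follows the player on X and Z within the bounds of its room.
; Construction sizes the confines box from room dimensions in 16-pixel units and places the player trigger box.
; BeginPlay caches the confine limits; Tick interpolates toward the player, clamps to them and moves the camera.
; Entering the trigger makes this the active camera with a cubic blend, or instantly if already overlapping at start.
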(event OnComponentBeginOverlap(PlayerTriggerBox)
  (params (OverlappedComponent :type Primitive%20Component%20Object%20Reference) (OtherActor :type Actor%20Object%20Reference) (OtherComp :type Primitive%20Component%20Object%20Reference) (OtherBodyIndex :type Integer) (bFromSweep :type Boolean) (SweepResult :type Hit%20Result%20Structure%20%28by%20ref%29))
  (bind _self self)
  ;[1 1 1] If Character Overlap TriggerBox, Set Active Camera
  (bind _asbp_paper_character (Utilities|Casting|CastToBP_PaperCharacter OtherActor))
  (Variables|/Game/Blueprints/BP_PaperCharacter.BP_PaperCharacter_C|SetCurrentCam _asbp_paper_character _self)
  (Game|Player|SetViewTargetwithBlend (Game|GetPlayerController 0) _self 0.6 "VTBlend_Cubic" 2.0 false))

(event EventBeginPlay
  (bind _self self)
  ;[1 1 1] On Begin Play If Character Collides with TriggerBox, Set Active Camera
  (Utilities|GetConfinesBoxBounds)
  (Utilities|FlowControl|Delay 0.0)
  (bind _asbp_paper_character (Utilities|Casting|CastToBP_PaperCharacter (Game|Player|GetPlayerPawn 0)))
  (for _array_element (Class|Actor|GetOverlappingComponents _asbp_paper_character)
    (if (== _array_element (Variables|Default|GetPlayerTriggerBox))
      (Variables|/Game/Blueprints/BP_PaperCharacter.BP_PaperCharacter_C|SetCurrentCam _asbp_paper_character _self)
      (Game|Player|SetViewTargetwithBlend (Game|GetPlayerController 0) _self 0.0 "VTBlend_Linear" 0.0 false))))

(event EventTick
  (params (DeltaSeconds :type Float%20%28single-precision%29))
  ;[1 1 1] Event Tick
  (Variables|Default|SetDeltaTime DeltaSeconds)
  (Utilities|FlowControl|Sequence
    (:then_0
      (Utilities|CamFollowPlayerX)
      (Utilities|CamFollowPlayerZ))
    (:then_1
      (Utilities|LerpWithinConfines)
      (Utilities|SetCameraPosition))))

(fn ConstructionScript
  (Transformation|SetRelativeTransform (Variables|Default|GetPlayerTriggerBox) (Variables|Trigger|GetPlayerTriggerTransform) false false)
  (Components|Box|SetBoxExtent (Variables|Default|GetPlayerTriggerBox) (Variables|Trigger|GetPlayerTriggerExtent) true)
  (Components|Box|SetBoxExtent (Variables|Default|GetCameraConfinesBox) (Math|Vector|MakeVector (Math|Conversions|ToFloat(Integer) (* (* (Variables|RoomSize|GetRoomWidth) 8) (Variables|RoomSize|GetRoomUnitWidth))) 1e+01 (Math|Conversions|ToFloat(Integer) (* (* (Variables|RoomSize|GetRoomHeight) 8) (Variables|RoomSize|GetRoomUnitHeigth)))) true))